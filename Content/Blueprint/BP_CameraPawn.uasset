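; Camera pawn that orbits its spring arm by left-mouse drag or single-finger touch drag and zooms with the mouse wheel.
; Mouse and touch deltas share one rotation path, adding yaw and inverted pitch, with pitch clamped to a downward-looking range.
; Tick detects two-finger touches to suppress touch-move rotation, but no pinch zoom is wired.
; Zoom adjusts arm length within fixed limits.
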(event EventBeginPlay)

(event Collision|EventActorBeginOverlap
  (params (OtherActor :type Actor%20Object%20Reference)))

(event EventTick
  (params (DeltaSeconds :type Float%20%28single-precision%29))
  (bind _returnvalue (Game|GetPlayerController 0))
  (bind _returnvalue_2 (Game|GetPlayerController 0))
  (bind _springarm (Variables|Default|GetSpringArm))
  (bind _currenttouchposition (Variables|Default|GetCurrentTouchPosition))
  (bind (_deltax _deltay) (Class|PlayerController|GetInputMouseDelta _returnvalue_2))
  (bind _relativerotation (Variables|/Script/Engine.SceneComponent|GetRelativeRotation _springarm))
  (Utilities|FlowControl|Sequence
    (:then_0
      (if (.bIsCurrentlyPressed (Class|PlayerController|GetInputTouchState _returnvalue "Touch1"))
        (if (.bIsCurrentlyPressed (Class|PlayerController|GetInputTouchState _returnvalue "Touch2"))
          (Variables|Default|SetCanPinch true)
          (else
            (Variables|Default|SetCanPinch false)))
        (else
          (Variables|Default|SetCanPinch false))))
    (:then_1
      (if (Game|Player|IsInputKeyDown _returnvalue_2 "LeftMouseButton")
        (Transformation|AddRelativeRotation _springarm (Math|Rotator|MakeRotator 0.0 (* (+ _deltay (.y (- (Math|Vector2D|MakeVector2D (.x _currenttouchposition) (.y _currenttouchposition)) (Math|Vector2D|MakeVector2D (.x (Variables|Default|GetPrevTouchPosition)) (.y (Variables|Default|GetPrevTouchPosition)))))) (Math|Float|MakeLiteralFloat -1.0)) (* (+ _deltax (.x (- (Math|Vector2D|MakeVector2D (.x _currenttouchposition) (.y _currenttouchposition)) (Math|Vector2D|MakeVector2D (.x (Variables|Default|GetPrevTouchPosition)) (.y (Variables|Default|GetPrevTouchPosition)))))) (Math|Float|MakeLiteralFloat 1.0))) false false)
        (Transformation|SetRelativeRotation _springarm (Math|Rotator|MakeRotator 0.0 (Math|Float|ClampAngle (.pitch _relativerotation) -8e+01 -3e+01) (.yaw _relativerotation)) false false)
        (Variables|Default|SetPrevTouchPosition (Variables|Default|GetCurrentTouchPosition))))
    (:then_2)))

(event Input|MouseEvents|MouseWheelAxis
  (params (AxisValue :type Float%20%28single-precision%29))
  (CallFunction|Zoom AxisValue -1.0))

(event Input|TouchEvents|InputTouch
  (params (Location :type Vector) (FingerIndex :type ETouchIndex%20Enum))
  (bind _returnvalue (Game|GetPlayerController 0))
  (bind _springarm (Variables|Default|GetSpringArm))
  (bind (_deltax _deltay) (Class|PlayerController|GetInputMouseDelta _returnvalue))
  (bind _relativerotation (Variables|/Script/Engine.SceneComponent|GetRelativeRotation _springarm))
  (:Pressed
    (bind _output_get (Variables|Default|SetPrevTouchPosition Location)))
  (:Released
    (Variables|Default|SetPrevTouchPosition "0, 0, 0")
    (Variables|Default|SetCurrentTouchPosition "0, 0, 0"))
  (:Moved
    (bind _output_get_2 (Variables|Default|SetCurrentTouchPosition Location))
    (if (> (Class|KismetMathLibrary|VectorDistanceSquared _output_get_2 _output_get) 15.0)
      (if (not (Variables|Default|GetCanPinch))
        (if (.bIsCurrentlyPressed (Class|PlayerController|GetInputTouchState (Game|GetPlayerController 0) "Touch1"))
          (Transformation|AddRelativeRotation _springarm (Math|Rotator|MakeRotator 0.0 (* (+ _deltay (.y (- (Math|Vector2D|MakeVector2D (.x (Variables|Default|GetCurrentTouchPosition)) (.y (Variables|Default|GetCurrentTouchPosition))) (Math|Vector2D|MakeVector2D (.x (Variables|Default|GetPrevTouchPosition)) (.y (Variables|Default|GetPrevTouchPosition)))))) (Math|Float|MakeLiteralFloat -1.0)) (* (+ _deltax (.x (- (Math|Vector2D|MakeVector2D (.x (Variables|Default|GetCurrentTouchPosition)) (.y (Variables|Default|GetCurrentTouchPosition))) (Math|Vector2D|MakeVector2D (.x (Variables|Default|GetPrevTouchPosition)) (.y (Variables|Default|GetPrevTouchPosition)))))) (Math|Float|MakeLiteralFloat 1.0))) false false)
          (Transformation|SetRelativeRotation _springarm (Math|Rotator|MakeRotator 0.0 (Math|Float|ClampAngle (.pitch _relativerotation) -8e+01 -3e+01) (.yaw _relativerotation)) false false)
          (Variables|Default|SetPrevTouchPosition (Variables|Default|GetCurrentTouchPosition)))))))

(fn ConstructionScript)

(fn Zoom
  (params (Zoom%20Value :type Float%20%28double-precision%29) (Dir :type Float%20%28double-precision%29))
  (bind _springarm (Variables|Default|GetSpringArm))
  (Variables|/Script/Engine.SpringArmComponent|SetTargetArmLength _springarm (Math|Float|Clamp(Float) (+ (Variables|/Script/Engine.SpringArmComponent|GetTargetArmLength _springarm) (* Zoom%20Value (* Dir 5e+01))) 4e+02 2.7e+03)))