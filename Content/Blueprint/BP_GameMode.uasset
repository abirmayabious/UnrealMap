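; BP_GameMode is a game mode whose SetActiveMesh function reveals the mesh actor matching a given index.
; It loops over actors tagged "Mesh" and reads each index through the BI_Mesh interface, unhiding matches.
; Only actors failing the interface cast get hidden, so non-matching BI_Mesh actors keep their current visibility.
; Debug prints trace the loop, while BeginPlay and Tick remain empty.
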(event EventBeginPlay)

(event EventTick
  (params (DeltaSeconds :type Float%20%28single-precision%29)))

(fn ConstructionScript)

(fn SetActiveMesh
  (params (MeshIndex :type Integer))
  (Development|PrintString "1")
  (bind _outactors (Actor|GetAllActorsOfClasswithTag "/Script/Engine.Actor" "Mesh"))
  (for _array_element _outactors
    (Development|PrintString (Utilities|GetDisplayName _array_element) true true "(R=1.000000,G=0.000000,B=0.192244,A=1.000000)")
    (bind _asbi_mesh (Utilities|Casting|CastToBI_Mesh _array_element)
      (:then
        (Development|PrintString "2")
        (bind _index (Default|GetIndex _asbi_mesh))
        (if (== MeshIndex _index)
          (Rendering|SetActorHiddenInGame _array_element false)))
      (:CastFailed
        (Rendering|SetActorHiddenInGame _array_element true)))))