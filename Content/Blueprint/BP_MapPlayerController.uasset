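; BP_MapPlayerController is a player controller that opens a map menu and reveals hidden cube or sphere actors.
; BeginPlay caches the first BP_SpawnedCube, then adds WBP_MapMenu with a visible cursor and Game-and-UI input, stopping early if that cast fails.
; SpawnedCube and SpawnedSphere events unhide their referenced actor and hide the menu, keeping the cursor visible.
; SphereRef is never assigned in this graph.
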(event Custom|SpawnedSphere
  (Rendering|SetActorHiddenInGame (Variables|Default|GetSphereRef) false)
  (Widget|SetVisibility (Variables|Default|GetMapWidget) "Hidden")
  (Variables|Default|SetbShowMouseCursor true)
  (Input|SetInputModeGameandUI self 0 "DoNotLock" false false))

(event Custom|SpawnedCube
  (Rendering|SetActorHiddenInGame (Variables|Default|GetCubeRef) false)
  (Widget|SetVisibility (Variables|Default|GetMapWidget) "Hidden")
  (Variables|Default|SetbShowMouseCursor true)
  (Input|SetInputModeGameandUI self 0 "DoNotLock" false false))

(event EventBeginPlay
  (Utilities|FlowControl|Sequence
    (:then_0
      (bind _outactors (Actor|GetAllActorsOfClass "/Game/Blueprint/BP_SpawnedCube.BP_SpawnedCube_C"))
      (bind _asbp_spawned_cube (Utilities|Casting|CastToBP_SpawnedCube (Utilities|Array|Get(acopy) _outactors)))
      (Variables|Default|SetCubeRef _asbp_spawned_cube)
      (bind _returnvalue (UserInterface|CreateWidget "/Game/Blueprint/WBP_MapMenu.WBP_MapMenu_C" self))
      (Variables|Default|SetMapWidget _returnvalue)
      (UserInterface|Viewport|AddtoViewport (Variables|Default|GetMapWidget) 0)
      (Variables|Default|SetbShowMouseCursor true)
      (Input|SetInputModeGameandUI self (Variables|Default|GetMapWidget) "DoNotLock" true false))))

(fn ConstructionScript)